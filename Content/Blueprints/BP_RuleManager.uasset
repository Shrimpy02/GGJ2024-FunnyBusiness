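; Rule manager that flags a clown as illegal when it carries a banned element, apparently an early prototype with debug-print output.
; BeginPlay adds the first ClownHats entry to IllegalElements.
; Each Tick finds a single BP_BaseClownCharacter, checks its actor tags against that list and prints on a match.
; An alternative per-mesh tag check on hat, body and face is present but disconnected.
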(event `Key|One`
  (params (Key :type "Key Structure"))
  (:`Pressed`
    (`KismetSystemLibrary.PrintString` "Hello")))

(event `self.ReceiveBeginPlay`
  (`KismetArrayLibrary.Array_Add` (`self.IllegalElements`) (`|GetArrayItem` (`self.ClownHats`))))

(event `self.ReceiveTick`
  (params (DeltaSeconds :type "Float (single-precision)"))
  (bind _returnvalue (`GameplayStatics.GetActorOfClass` "/Game/Characters/BP_BaseClownCharacter.BP_BaseClownCharacter_C"))
  (if (> (`KismetArrayLibrary.Array_Length` (`self.IllegalElements`)) 0)
    (for _index (range (`KismetArrayLibrary.Array_Length` (`self.IllegalElements`)))
      (set `self.ThisClownIsIllegal` (`self.ActorHasTag` _returnvalue (`|GetArrayItem` (`self.IllegalElements`) _index)))
      (if (`self.ThisClownIsIllegal`)
        (`KismetSystemLibrary.PrintString` "Eligual")))))

(fn `UserConstructionScript`)