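; BP_ClownDebugClass is a debug Blueprint that displays a clown's torso, pants and hat numbers as text.
; Every Tick, it converts the three integer variables to text and pushes each into its matching text element.
; The graph never sets those integers itself, and its construction script is empty.
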(event `self.ReceiveTick`
  (params (DeltaSeconds :type "Float (single-precision)"))
  (`TextRenderComponent.K2_SetText` (`self.Torso Number`) (`KismetTextLibrary.Conv_IntToText` (`self.clownTorsoInt`)))
  (`TextRenderComponent.K2_SetText` (`self.Pants Number`) (`KismetTextLibrary.Conv_IntToText` (`self.clownPantsInt`)))
  (`TextRenderComponent.K2_SetText` (`self.Hat Number`) (`KismetTextLibrary.Conv_IntToText` (`self.clownHatInt`))))

(fn `UserConstructionScript`)