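; Base clown character that animates in, crosses the scene and destroys itself, with a randomized look.
; On BeginPlay a timeline moves and scales it, then Tick starts a sideways timeline that ends in destruction.
; Hat, face and body get random materials, plus BP_RuleManager tags from separate random rolls, so tags may not match visuals.
; On destruction it refreshes the joke sheet with a generated joke and triggers a new rule on WBP_MainScene.
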(event `self.ReceiveBeginPlay`
  (bind (_returnvalue_x _returnvalue_y _returnvalue_z) (`KismetMathLibrary.BreakVector` (`self.K2_GetActorLocation`)))
  (`|ExecutionSequence`
    (:`then_0`
      (set `self.MoveComplete` false)
      (set `self.ScaleComplete` false)
      (bind (_direction _scale _location) (`Timeline|Timeline`)
        (:`Update`
          (`SceneComponent.K2_SetRelativeLocation` (`self.TheRoot`) (`KismetMathLibrary.MakeVector` _returnvalue_x _returnvalue_y _location) false false)
          (`SceneComponent.SetRelativeScale3D` (`self.TheRoot`) (`KismetMathLibrary.Conv_DoubleToVector` _scale)))
        (:`Finished`
          (set `self.ScaleComplete` true))))
    (:`then_1`
      (`KismetArrayLibrary.Array_Add` (`self.Tags`) "Top hat"))
    (:`then_2`
      (`self.GetRandomMaterialToMesh`))))

(event `self.ReceiveTick`
  (params (DeltaSeconds :type "Float (single-precision)"))
  (bind (_returnvalue_x _returnvalue_y _returnvalue_z) (`KismetMathLibrary.BreakVector` (`self.K2_GetActorLocation`)))
  (`|ExecutionSequence`
    (:`then_0`
      (if (`self.ScaleComplete`)
        (bind (_direction _location) (`Timeline|Timeline_0`)
          (:`Update`
            (`SceneComponent.K2_SetRelativeLocation` (`self.TheRoot`) (`KismetMathLibrary.MakeVector` _returnvalue_x _location _returnvalue_z) false false))
          (:`Finished`
            (set `self.MoveComplete` true)))))
    (:`then_1`
      (if (`self.MoveComplete`)
        (`self.K2_DestroyActor`)))))

(event `GetRandomMaterialToMesh`
  (bind _facemesh (`self.FaceMesh`))
  (bind _bodymesh (`self.BodyMesh`))
  (bind _componenttags (`ActorComponent.ComponentTags` _bodymesh))
  (bind _componenttags_2 (`ActorComponent.ComponentTags` (`self.HatMesh`)))
  (`|ExecutionSequence`
    (:`then_0`
      (bind _returnvalue (`GameplayStatics.GetActorOfClass` "/Game/Blueprints/BP_RuleManager.BP_RuleManager_C"))
      (bind _returnvalue_2 (`KismetMathLibrary.RandomIntegerInRange` 0 (- (`KismetArrayLibrary.Array_Length` (`RuleManager.ClownHats` _returnvalue)) 1)))
      ;[1 1 1] Hats
      (switch `int` _returnvalue_2
        (:`0`
          (`PrimitiveComponent.SetMaterial` (`self.HatMesh`) 0 "/Game/Assets/Characters/Hat/Woman/HeadJudge.HeadJudge")
          (bind _output (`|GetArrayItem` (`RuleManager.ClownHats` _returnvalue) _returnvalue_2))
          (`KismetArrayLibrary.Array_Add` _componenttags_2 _output))
        (:`1`
          (`PrimitiveComponent.SetMaterial` (`self.HatMesh`) 0 "/Game/Assets/Characters/Hat/Woman/HeadPaperHat.HeadPaperHat")
          (`KismetArrayLibrary.Array_Add` _componenttags_2 _output))
        (:`2`
          (`PrimitiveComponent.SetMaterial` (`self.HatMesh`) 0 "/Game/Assets/Characters/Hat/Woman/HeadPinkHair.HeadPinkHair")
          (`KismetArrayLibrary.Array_Add` _componenttags_2 _output))
        (:`3`
          (`PrimitiveComponent.SetMaterial` (`self.HatMesh`) 0 "/Game/Assets/Characters/Hat/Woman/HeadRainbow.HeadRainbow")
          (`KismetArrayLibrary.Array_Add` _componenttags_2 _output))
        (:`4`
          (`PrimitiveComponent.SetMaterial` (`self.HatMesh`) 0 "/Game/Assets/Characters/Hat/Woman/HeadPurpleJester.HeadPurpleJester")
          (`KismetArrayLibrary.Array_Add` _componenttags_2 _output))))
    (:`then_1`
      (bind _returnvalue_3 (`GameplayStatics.GetActorOfClass` "/Game/Blueprints/BP_RuleManager.BP_RuleManager_C"))
      (bind _returnvalue_4 (`KismetMathLibrary.RandomIntegerInRange` 0 (- (`KismetArrayLibrary.Array_Length` (`RuleManager.ClownFaces` _returnvalue_3)) 1)))
      ;[1 1 1] Face
      (switch `int` _returnvalue_4
        (:`0`
          (`PrimitiveComponent.SetMaterial` _facemesh 0 "/Game/Assets/Characters/Face/Woman/FaceChipsFace.FaceChipsFace")
          (bind _output_2 (`|GetArrayItem` (`RuleManager.ClownFaces` _returnvalue_3) _returnvalue_4))
          (`KismetArrayLibrary.Array_Add` (`ActorComponent.ComponentTags` _facemesh) _output_2))
        (:`1`
          (`PrimitiveComponent.SetMaterial` _facemesh 0 "/Game/Assets/Characters/Face/Woman/FaceJoker.FaceJoker")
          (`KismetArrayLibrary.Array_Add` (`ActorComponent.ComponentTags` _facemesh) _output_2))
        (:`2`
          (`PrimitiveComponent.SetMaterial` _facemesh 0 "/Game/Assets/Characters/Face/Woman/FacePigNose.FacePigNose")
          (`KismetArrayLibrary.Array_Add` (`ActorComponent.ComponentTags` _facemesh) _output_2))
        (:`3`
          (`PrimitiveComponent.SetMaterial` _facemesh 0 "/Game/Assets/Characters/Face/Woman/FacePurpleEye.FacePurpleEye")
          (`KismetArrayLibrary.Array_Add` (`ActorComponent.ComponentTags` _facemesh) _output_2))
        (:`4`
          (`PrimitiveComponent.SetMaterial` _facemesh 0 "/Game/Assets/Characters/Face/Woman/FaceRedDots.FaceRedDots")
          (`KismetArrayLibrary.Array_Add` (`ActorComponent.ComponentTags` _facemesh) _output_2))
        (:`5`
          (`PrimitiveComponent.SetMaterial` _facemesh 0 "/Game/Assets/Characters/Face/Woman/FaceRedNose.FaceRedNose")
          (`KismetArrayLibrary.Array_Add` (`ActorComponent.ComponentTags` _facemesh) _output_2))
        (:`6`
          (`PrimitiveComponent.SetMaterial` _facemesh 0 "/Game/Assets/Characters/Face/Woman/FaceSpookyAF.FaceSpookyAF")
          (`KismetArrayLibrary.Array_Add` (`ActorComponent.ComponentTags` _facemesh) _output_2))))
    (:`then_2`
      (bind _returnvalue_5 (`GameplayStatics.GetActorOfClass` "/Game/Blueprints/BP_RuleManager.BP_RuleManager_C"))
      (bind _returnvalue_6 (`KismetMathLibrary.RandomIntegerInRange` 0 (- (`KismetArrayLibrary.Array_Length` (`RuleManager.ClownClothes` _returnvalue_5)) 1)))
      ;[1 1 1] Body
      (switch `int` _returnvalue_6
        (:`0`
          (`PrimitiveComponent.SetMaterial` _bodymesh 0 "/Game/Assets/Characters/Body/Woman/BodyClown.BodyClown")
          (bind _output_3 (`|GetArrayItem` (`RuleManager.ClownClothes` _returnvalue_5) _returnvalue_6))
          (`KismetArrayLibrary.Array_Add` _componenttags _output_3))
        (:`1`
          (`PrimitiveComponent.SetMaterial` _bodymesh 0 "/Game/Assets/Characters/Body/Woman/BodyGGJ.BodyGGJ")
          (`KismetArrayLibrary.Array_Add` _componenttags _output_3))
        (:`2`
          (`PrimitiveComponent.SetMaterial` _bodymesh 0 "/Game/Assets/Characters/Body/Woman/BodyJester.BodyJester")
          (`KismetArrayLibrary.Array_Add` _componenttags _output_3))
        (:`3`
          (`PrimitiveComponent.SetMaterial` _bodymesh 0 "/Game/Assets/Characters/Body/Woman/BodyPinkDress.BodyPinkDress")
          (`KismetArrayLibrary.Array_Add` _componenttags _output_3))
        (:`4`
          (`PrimitiveComponent.SetMaterial` _bodymesh 0 "/Game/Assets/Characters/Body/Woman/BodyPrisonUniform.BodyPrisonUniform")
          (`KismetArrayLibrary.Array_Add` _componenttags _output_3))
        (:`5`
          (`PrimitiveComponent.SetMaterial` _bodymesh 0 "/Game/Assets/Characters/Body/Woman/BodyRaincoat.BodyRaincoat")
          (`KismetArrayLibrary.Array_Add` _componenttags _output_3))
        (:`6`
          (`PrimitiveComponent.SetMaterial` _bodymesh 0 "/Game/Assets/Characters/Body/Woman/BodyWifeBeater.BodyWifeBeater")
          (`KismetArrayLibrary.Array_Add` _componenttags _output_3))))))

(event `self.ReceiveDestroyed`
  (`|ExecutionSequence`
    (:`then_0`
      (bind _foundwidgets (`WidgetBlueprintLibrary.GetAllWidgetsOfClass` "/Game/Blueprints/InGame/WBP_JokeSheet.WBP_JokeSheet_C"))
      (if (`KismetArrayLibrary.Array_IsValidIndex` _foundwidgets)
        (bind _returnvalue (`GameplayStatics.GetActorOfClass` "/Game/Blueprints/BP_RuleManager.BP_RuleManager_C"))
        (bind _returnvalue_2 (`RuleManager.generateJokeSentance` _returnvalue))
        (`/Game/Blueprints/InGame/WBP_JokeSheet.SetCurrentJoke` (`|GetArrayItem` _foundwidgets) _returnvalue_2)))
    (:`then_1`
      (bind _foundwidgets_2 (`WidgetBlueprintLibrary.GetAllWidgetsOfClass` "/Game/Blueprints/InGame/WBP_JokeSheetOpen.WBP_JokeSheetOpen_C"))
      (if (`KismetArrayLibrary.Array_IsValidIndex` _foundwidgets_2)
        (`Widget.RemoveFromParent` (`|GetArrayItem` _foundwidgets_2))
        (bind _returnvalue_3 (`|CreateWidget` "/Game/Blueprints/InGame/WBP_JokeSheet.WBP_JokeSheet_C"))
        (`UserWidget.AddToViewport` _returnvalue_3 0)
        (bind _returnvalue_4 (`GameplayStatics.GetActorOfClass` "/Game/Blueprints/BP_RuleManager.BP_RuleManager_C"))
        (bind _returnvalue_5 (`RuleManager.generateJokeSentance` _returnvalue_4))
        (`/Game/Blueprints/InGame/WBP_JokeSheet.SetCurrentJoke` _returnvalue_3 _returnvalue_5)))
    (:`then_2`
      (bind _foundwidgets_3 (`WidgetBlueprintLibrary.GetAllWidgetsOfClass` "/Game/Blueprints/InGame/WBP_MainScene.WBP_MainScene_C"))
      (if (`KismetArrayLibrary.Array_IsValidIndex` _foundwidgets_3)
        (`/Game/Blueprints/InGame/WBP_MainScene.new rule!` (`|GetArrayItem` _foundwidgets_3))
        (bind _returnvalue_6 (`|CreateWidget` "/Game/Blueprints/InGame/WBP_NewRule.WBP_NewRule_C"))
        (`UserWidget.AddToViewport` _returnvalue_6 0)))))

(fn `UserConstructionScript`)