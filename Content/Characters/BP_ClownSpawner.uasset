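; BP_ClownSpawner is an actor that triggers clown spawning and also sets up the pause menu when play begins.
; BeginPlay creates and stores a PauseMenuWidget without adding it to the viewport, then hides the cursor, disables click and mouse-over events and switches to game-only input.
; A DoOnce then calls SpawnClowns, followed by a Delay that leads nowhere, so no repeat happens here.
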(event `self.ReceiveBeginPlay`
  (bind _returnvalue (`GameplayStatics.GetPlayerController` 0))
  (bind _returnvalue_2 (`|CreateWidget` "/Game/Blueprints/PauseMenuWidget.PauseMenuWidget_C" (`GameplayStatics.GetPlayerController` 0)))
  (bind _output_get (set `self.Pause Screen` _returnvalue_2))
  (set `/Game/Blueprints/PauseMenuWidget.PlayerActor` _output_get _returnvalue_2)
  (bind _output_get_2 (set `PlayerController.bShowMouseCursor` false _returnvalue))
  (bind _output_get_3 (set `PlayerController.bEnableClickEvents` _output_get_2 _returnvalue))
  (set `PlayerController.bEnableMouseOverEvents` _output_get_3 _returnvalue)
  (`WidgetBlueprintLibrary.SetInputMode_GameOnly` _returnvalue)
  (`/Engine/EditorBlueprintResources/StandardMacros.DoOnce` false
    (:`Completed`
      (`self.SpawnClowns` null)
      (`KismetSystemLibrary.Delay` 12.0))))

(event `self.ReceiveTick`
  (params (DeltaSeconds :type "Float (single-precision)")))

(fn `UserConstructionScript`)